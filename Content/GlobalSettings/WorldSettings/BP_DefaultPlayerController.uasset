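; Default player controller that relays player stat changes to the HUD.
; On BeginPlay it casts the HUD to BP_PlayerUI and caches it.
; Custom events set max health, stamina and mask power directly, and forward current health, stamina, mask power, predicted health and stored power to the HUD's update functions.
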(event `self.ReceiveBeginPlay`
  ;[1 1 1] Init
  (bind _asbp_player_ui (cast `/Game/GlobalSettings/WorldSettings/BP_PlayerUI` (`self.GetHUD`)))
  (set `self.PlayerUI` _asbp_player_ui))

(event `/Game/GlobalSettings/Interfaces/BPI_PlayerController.UpdateMaxStaminaUI`
  (params (Stamina :type "Float (single-precision)"))
  ;[1 0.5 0] Stamina
  (set `/Game/GlobalSettings/WorldSettings/BP_PlayerUI.MaxStamina` Stamina (`self.PlayerUI`)))

(event `/Game/GlobalSettings/Interfaces/BPI_PlayerController.UpdateMaxHealthUI`
  (params (Health :type "Float (single-precision)"))
  ;[0 1 0] Health
  (set `/Game/GlobalSettings/WorldSettings/BP_PlayerUI.MaxHealth` Health (`self.PlayerUI`)))

(event `/Game/GlobalSettings/Interfaces/BPI_PlayerController.UpdateMaxMaskPowerUI`
  (params (MaskPower :type "Float (single-precision)"))
  ;[0.5 0 1] Mask
  (set `/Game/GlobalSettings/WorldSettings/BP_PlayerUI.MaxMaskPower` MaskPower (`self.PlayerUI`)))

(event `/Game/GlobalSettings/Interfaces/BPI_PlayerController.UpdateStaminaUI`
  (params (Stamina :type "Float (single-precision)"))
  ;[1 0.5 0] Stamina
  (`/Game/GlobalSettings/WorldSettings/BP_PlayerUI.UpdateStamina` (`self.PlayerUI`) Stamina))

(event `/Game/GlobalSettings/Interfaces/BPI_PlayerController.UpdateHealthUI`
  (params (Health :type "Float (single-precision)"))
  ;[0 1 0] Health
  (`/Game/GlobalSettings/WorldSettings/BP_PlayerUI.UpdateHealth` (`self.PlayerUI`) Health))

(event `/Game/GlobalSettings/Interfaces/BPI_PlayerController.UpdateMaskPowerUI`
  (params (MaskPower :type "Float (single-precision)"))
  ;[0.5 0 1] Mask
  (`/Game/GlobalSettings/WorldSettings/BP_PlayerUI.UpdateMaskPower` (`self.PlayerUI`) MaskPower))

(event `/Game/GlobalSettings/Interfaces/BPI_PlayerController.UpdatePredictedHealthUI`
  (params (Health :type "Float (single-precision)"))
  ;[0 1 0] Health
  (`/Game/GlobalSettings/WorldSettings/BP_PlayerUI.UpdatePredictedHealth` (`self.PlayerUI`) Health))

(event `/Game/GlobalSettings/Interfaces/BPI_PlayerController.UpdateStoredPowerUI`
  (params (StoredPower :type Integer))
  ;[0.5 0 1] Mask
  (`/Game/GlobalSettings/WorldSettings/BP_PlayerUI.UpdateStoredPower` (`self.PlayerUI`) StoredPower))

(fn `UserConstructionScript`)