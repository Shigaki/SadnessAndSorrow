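; Player UI manager that owns the on-screen stats bar and the player menu.
; BeginPlay creates both widgets but shows only the stats bar, which update events fill with health, predicted health, stamina, mask power and stored power.
; ToggleMenu opens or closes the menu and switches its submenus by mapping the requested menu to a child index, collapsing the rest, and returns whether the menu is open.
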(event `self.ReceiveBeginPlay`
  ;[1 1 1] Init
  (bind _returnvalue (`|CreateWidget` "/Game/UI/PlayerInfo/StatsBar.StatsBar_C" (`self.GetOwningPlayerController`)))
  (bind _output_get (set `self.StatsBar` _returnvalue))
  (`UserWidget.AddToViewport` _output_get 0)
  (bind _returnvalue_2 (`|CreateWidget` "/Game/UI/PlayerMenu/W_PlayerMenu.W_PlayerMenu_C"))
  (set `self.PlayerMenu` _returnvalue_2))

(event `UpdateHealth`
  (params (Health :type "Float (double-precision)"))
  (bind _statsbar (`self.StatsBar`))
  ;[0 1 0] Health
  (`TextBlock.SetText` (`/Game/UI/PlayerInfo/StatsBar.T_CurrentHealth` _statsbar) (`KismetTextLibrary.Conv_DoubleToText` Health "HalfToEven"))
  (`ProgressBar.SetPercent` (`/Game/UI/PlayerInfo/StatsBar.PB_CurrentHealth` _statsbar) (/ Health (`self.MaxHealth`))))

(event `UpdateStamina`
  (params (Stamina :type "Float (double-precision)"))
  ;[1 0.5 0] Stamina
  (`ProgressBar.SetPercent` (`/Game/UI/PlayerInfo/StatsBar.PB_Stamina` (`self.StatsBar`)) (/ Stamina (`self.MaxStamina`))))

(event `UpdatePredictedHealth`
  (params (Health :type "Float (double-precision)"))
  ;[0 1 0] Health
  (`ProgressBar.SetPercent` (`/Game/UI/PlayerInfo/StatsBar.PB_PredictedHealth` (`self.StatsBar`)) (/ Health (`self.MaxHealth`))))

(event `UpdateMaskPower`
  (params (MaskPower :type "Float (double-precision)"))
  ;[0.5 0 1] Mask
  (`ProgressBar.SetPercent` (`/Game/UI/PlayerInfo/StatsBar.PB_Mask` (`self.StatsBar`)) (/ MaskPower (`self.MaxMaskPower`))))

(event `UpdateStoredPower`
  (params (StoredPower :type Integer))
  ;[0.5 0 1] Mask
  ;;[1 1 1] Change to VFX
  (`TextBlock.SetText` (`/Game/UI/PlayerInfo/StatsBar.T_StoredPower` (`self.StatsBar`)) (`KismetTextLibrary.Conv_IntToText` StoredPower)))

(fn `ToggleMenu`
  (params (Menu :type "/Game/GlobalSettings/Enums/E_SubMenu Enum" :default "NewEnumerator0"))
  (returns (ShowCursor :type Boolean))
  (locals (DesiredMenu :type "/Game/GlobalSettings/Enums/E_SubMenu Enum" :default "NewEnumerator0") (ShowSubMenu :type Boolean))
  (set `local.DesiredMenu` Menu)
  (if (`Widget.IsInViewport` (`self.PlayerMenu`))
    (if (`|EnumEquality` (`local.DesiredMenu`) "NewEnumerator6")
      (`Widget.RemoveFromParent` (`self.PlayerMenu`))
      (return false)
      (else
        (set `local.ShowSubMenu` (not (`Widget.IsVisible` (`PanelWidget.GetChildAt` (`/Game/UI/PlayerMenu/W_PlayerMenu.SubMenu` (`self.PlayerMenu`)) (select `/Game/GlobalSettings/Enums/E_SubMenu` (`local.DesiredMenu`) :`NewEnumerator1` 1 :`NewEnumerator2` 2 :`NewEnumerator3` 3 :`NewEnumerator4` 4 :`NewEnumerator5` 5)))))
        (for _array_element (`PanelWidget.GetAllChildren` (`/Game/UI/PlayerMenu/W_PlayerMenu.SubMenu` (`self.PlayerMenu`)))
          (`Widget.SetVisibility` _array_element "Collapsed"))
        (if (`local.ShowSubMenu`)
          (`Widget.SetVisibility` (`PanelWidget.GetChildAt` (`/Game/UI/PlayerMenu/W_PlayerMenu.SubMenu` (`self.PlayerMenu`)) (select `/Game/GlobalSettings/Enums/E_SubMenu` (`local.DesiredMenu`) :`NewEnumerator1` 1 :`NewEnumerator2` 2 :`NewEnumerator3` 3 :`NewEnumerator4` 4 :`NewEnumerator5` 5)) "Visible"))
        (return true)))
    (else
      (`Widget.SetVisibility` (`self.PlayerMenu`) "Visible")
      (for _array_element_2 (`PanelWidget.GetAllChildren` (`/Game/UI/PlayerMenu/W_PlayerMenu.SubMenu` (`self.PlayerMenu`)))
        (`Widget.SetVisibility` _array_element_2 "Collapsed"))
      (if (not (`|EnumEquality` (`local.DesiredMenu`) "NewEnumerator6"))
        (`Widget.SetVisibility` (`PanelWidget.GetChildAt` (`/Game/UI/PlayerMenu/W_PlayerMenu.SubMenu` (`self.PlayerMenu`)) (select `/Game/GlobalSettings/Enums/E_SubMenu` (`local.DesiredMenu`) :`NewEnumerator1` 1 :`NewEnumerator2` 2 :`NewEnumerator3` 3 :`NewEnumerator4` 4 :`NewEnumerator5` 5)) "Visible"))
      (`UserWidget.AddToViewport` (`self.PlayerMenu`) 0)
      (return true))))

(fn `UserConstructionScript`)