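; BPC_EnemyTest is a test enemy AI controller that runs the BT_EnemyAI behavior tree on possession.
; It exposes setter functions that write target actor, line of sight, hit reaction and death state to the Blackboard, using key-name variables.
; The death setter only sets its flag to true, and the file itself contains no perception or decision logic.
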(event `self.ReceivePossess`
  (params (PossessedPawn :type "Pawn Object Reference"))
  (`self.RunBehaviorTree` "/Game/Characters/Monsters/EnemyAITest/BT_EnemyAI.BT_EnemyAI"))

(fn `SetIsDead`
  (`BlackboardComponent.SetValueAsBool` (`self.Blackboard`) (`self.isDeadName`) true))

(fn `UpdateHasLineOfSightKey`
  (params (HasLineOfSight :type Boolean))
  (`BlackboardComponent.SetValueAsBool` (`self.Blackboard`) (`self.HasLineOfSightName`) HasLineOfSight))

(fn `UpdateReactToHit`
  (params (Hit :type Boolean))
  (`BlackboardComponent.SetValueAsBool` (`self.Blackboard`) (`self.ReactToHitName`) Hit))

(fn `UpdateTargetActorKey`
  (params (TargetActor :type "Actor Object Reference"))
  (`BlackboardComponent.SetValueAsObject` (`self.Blackboard`) (`self.TargetActorName`) TargetActor))

(fn `UserConstructionScript`)