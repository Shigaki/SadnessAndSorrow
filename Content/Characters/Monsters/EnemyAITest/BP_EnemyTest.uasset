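; BP_EnemyTest is a test monster enemy that perceives targets, reacts to damage and performs a punch attack.
; AI perception pushes target and line-of-sight keys to its BPC_EnemyTest controller, with a short timer delaying target clearing after sensing fails.
; Damage while alive sets the controller's hit-reaction key.
; Attack plays a punch montage, while CheckHit sphere-traces forward from a hand socket to apply damage.
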(event `self.AIPerception.OnTargetPerceptionUpdated`
  (params (Actor :type "Actor Object Reference") (Stimulus :type "AIStimulus Structure"))
  (set `self.PerceivedActor` Actor)
  (if (`.bSuccessfullySensed` (break `AIStimulus` Stimulus))
    (`KismetSystemLibrary.K2_ClearAndInvalidateTimerHandle` (`self.TargetLostTimer`))
    (bind _asbpc_enemy_test (cast `/Game/Characters/Monsters/EnemyAITest/BPC_EnemyTest` (`self.GetController`)))
    (`/Game/Characters/Monsters/EnemyAITest/BPC_EnemyTest.UpdateTargetActorKey` _asbpc_enemy_test (`self.PerceivedActor`))
    (bind _asbpc_enemy_test_2 (cast `/Game/Characters/Monsters/EnemyAITest/BPC_EnemyTest` (`self.GetController`)))
    (`/Game/Characters/Monsters/EnemyAITest/BPC_EnemyTest.UpdateHasLineOfSightKey` _asbpc_enemy_test_2 true)
    (else
      (bind _returnvalue (`KismetSystemLibrary.K2_SetTimerDelegate` (delegate `TargetLost`) 3.0))
      (set `self.TargetLostTimer` _returnvalue)
      (bind _asbpc_enemy_test_3 (cast `/Game/Characters/Monsters/EnemyAITest/BPC_EnemyTest` (`self.GetController`)))
      (`/Game/Characters/Monsters/EnemyAITest/BPC_EnemyTest.UpdateHasLineOfSightKey` _asbpc_enemy_test_3 false))))

(event `TargetLost`
  (set `self.PerceivedActor` null)
  (bind _asbpc_enemy_test (cast `/Game/Characters/Monsters/EnemyAITest/BPC_EnemyTest` (`self.GetController`)))
  (`/Game/Characters/Monsters/EnemyAITest/BPC_EnemyTest.UpdateTargetActorKey` _asbpc_enemy_test null))

(event `self.AIPerception.OnPerceptionUpdated`
  (params (UpdatedActors :type "Array of Actor Object Reference (by ref)")))

(event `self.ReceiveAnyDamage`
  (params (Damage :type "Float (single-precision)") (DamageType :type "DamageType Object Reference") (InstigatedBy :type "Controller Object Reference") (DamageCauser :type "Actor Object Reference"))
  (`parent.ReceiveAnyDamage` Damage DamageType InstigatedBy DamageCauser)
  (if (`self.isAlive`)
    (bind _output_get (set `self.bReactToHit` true))
    (bind _asbpc_enemy_test (cast `/Game/Characters/Monsters/EnemyAITest/BPC_EnemyTest` (`self.GetController`)))
    (`/Game/Characters/Monsters/EnemyAITest/BPC_EnemyTest.UpdateReactToHit` _asbpc_enemy_test _output_get)))

(event `Attack`
  (`self.PlayAnimMontage` "/Game/Characters/Monsters/EnemyAITest/Mutant_Punch_Montage.Mutant_Punch_Montage"))

(event `CheckHit`
  (bind _returnvalue (`SceneComponent.GetSocketLocation` (`self.Mesh`) "HitSocket"))
  (bind _outhit (`KismetSystemLibrary.SphereTraceSingle` :`Start` _returnvalue :`End` (+ _returnvalue (* (`KismetMathLibrary.GetForwardVector` (`self.K2_GetActorRotation`)) 100.0)) :`Radius` 40.0 :`TraceChannel` "TraceTypeQuery2" :`DrawDebugType` "ForOneFrame"))
  (`GameplayStatics.ApplyDamage` (`.HitActor` (`GameplayStatics.BreakHitResult` _outhit)) 50.0 null self "/Script/Engine.DamageType"))

(fn `UserConstructionScript`
  (`parent.UserConstructionScript`))