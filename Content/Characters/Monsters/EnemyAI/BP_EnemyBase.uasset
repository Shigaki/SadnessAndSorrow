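; Base enemy monster Blueprint that roams around its spawn point and fights a player once given a target.
; In combat it faces the target, taunts, then loops chasing and distance-based attack picks (light, heavy, charge or ranged) timed by random montage lengths.
; Authority-checked melee overlaps and forward sphere hits apply per-type damage, with knockback on sphere hits, while ranged attacks spawn projectiles.
; A looping timer calls target clearing when the player gets too far.
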(event `Multiplayer_PlayMontage`
  (params (InSkeletalMeshComponent :type "SkeletalMeshComponent Object Reference") (MontageToPlay :type "AnimMontage Object Reference") (StartingSection :type Name))
  ;[1 1 1 1 36] Multiplayer
  (`|PlayMontage` InSkeletalMeshComponent MontageToPlay 1.0 0.0 StartingSection))

(event `ClearPlayerTarget_1_1`
  ;[1 0.0449 0 1 36] ClearTarget
  (set `self.InCombat` false)
  (`self.SetActorTickEnabled` false)
  (set `self.Target` null)
  (`self.ClearPlayerTarget`)
  (`|AIMoveTo` self (`self.SpawnLocation`) null
    (:`OnSuccess`
      (`self.SetRoaming`))
    (:`OnFail`
      (`self.K2_SetActorLocation` (`self.SpawnLocation`))
      (`self.SetRoaming`))))

(event `self.ReceiveBeginPlay`
  ;[1 0.0549 0 1 36] BeginPlay
  ;;[0 0 0] StartRoaming
  (set `self.SpawnLocation` (`self.K2_GetActorLocation`))
  (`KismetSystemLibrary.Delay` 0.5)
  (`self.SetRoaming`))

(event `self.SetRoaming`
  ;[0 0.3317 1 1 32] Roaming
  (if (and (not (`self.IsRoaming`)) (not (`self.InCombat`)))
    (`self.MovmentState` "NewEnumerator1")
    (`|AIMoveTo` self (`NavigationSystemV1.K2_GetRandomReachablePointInRadius` (`self.SpawnLocation`) 1000.0 null null) null 1500.0
      (:`then`
        (set `self.IsRoaming` true))
      (:`OnSuccess`
        (set `self.IsRoaming` false)
        (`KismetSystemLibrary.Delay` 0.5)
        (`self.SetRoaming`)))))

(event `self.PlayerTarget`
  (params (Target :type "Actor Object Reference"))
  ;[0 0.3505 1 1 32] Set Player Target
  (set `self.Target` Target)
  (set `self.InCombat` true)
  (set `self.IsRoaming` false)
  (`self.SetActorTickEnabled` true)
  (set `self.CombatLocation` (`self.K2_GetActorLocation`))
  (`self.MovmentState` "NewEnumerator2")
  (`self.CheckTaunt`)
  (bind _returnvalue (`KismetSystemLibrary.K2_SetTimer` null "DistanceCheck" 1.0 true))
  (set `self.DistanceHandle` _returnvalue))

(event `self.ReceiveTick`
  (params (DeltaSeconds :type "Float (single-precision)"))
  (bind (_returnvalue_roll _returnvalue_pitch _returnvalue_yaw) (`KismetMathLibrary.BreakRotator` (`KismetMathLibrary.FindLookAtRotation` (`self.K2_GetActorLocation`) (`self.K2_GetActorLocation` (`self.Target`)))))
  ;[0 0.3505 1 1 32] Set Player Target
  ;;[0 0.02987 0.151] Rotate to Player
  (if (`self.InCombat`)
    (`self.Target`
      (:`then`
        (`self.K2_SetActorRotation` (`KismetMathLibrary.MakeRotator` 0.0 0.0 _returnvalue_yaw)))
      (:`else`))))

(event `self.CheckTaunt`
  (bind _output (`self.GetMontage` (`self.TauntMontage`)))
  ;[0 0.3505 1 1 32] Set Player Target
  ;;[0 0.07112 0.2917] Taunt with Agro
  (`Controller.StopMovement` (`self.GetController`))
  (if (> (`self.GetDistanceTo` self (`self.Target`)) 100.0)
    (`self.Multiplayer_PlayMontage` null _output)
    (bind _returnvalue (`AnimSequenceBase.GetPlayLength` _output))
    (`KismetSystemLibrary.Delay` _returnvalue)
    (`self.ChasePlayer`)
    (else
      (`self.ChasePlayer`))))

(event `self.ChasePlayer`
  ;[0 0.2882 1] Chasing Player
  ;[0 0.2882 1] Chasing Player
  (if (`self.InCombat`)
    (bind _lenght (`self.PickAttack` (`self.GetDistanceTo` self (`self.Target`))))
    (`KismetSystemLibrary.Delay` (+ _lenght 0.5))
    (`|AIMoveTo` self (0.0 0.0 0.0) (`self.Target`) 50.0
      (:`OnSuccess`
        (`self.AttackChoices`))
      (:`OnFail`
        (`KismetSystemLibrary.PrintString` "FailedToGetPlayer" true true (struct :`R` 1.0 :`A` 1.0))
        (`self.ClearPlayerTarget`)))))

(event `self.AttackChoices`
  ;[1 0.01884 0.07856] PickAttack
  (`self.Target`
    (:`then`
      (if true
        (bind _lenght (`self.PickAttack` (`self.GetDistanceTo` self (`self.Target`))))
        (`KismetSystemLibrary.Delay` (+ _lenght 0.5))
        (`self.ChasePlayer`)
        (else
          (`self.ClearPlayerTarget`))))
    (:`else`
      (`self.ClearPlayerTarget`))))

(event `self.MelleCollision`
  (params (State :type Boolean))
  ;[0 0.2583 1] SettingMelle Collision
  (if State
    (`PrimitiveComponent.SetCollisionEnabled` (`self.MelleTargetRange`) "QueryOnly")
    (else
      (`PrimitiveComponent.SetCollisionEnabled` (`self.MelleTargetRange`) "NoCollision"))))

(event `self.MelleTargetRange.OnComponentBeginOverlap`
  (params (OverlappedComponent :type "PrimitiveComponent Object Reference") (OtherActor :type "Actor Object Reference") (OtherComp :type "PrimitiveComponent Object Reference") (OtherBodyIndex :type Integer) (bFromSweep :type Boolean) (SweepResult :type "HitResult Structure (by ref)"))
  ;[0 0.2867 1] Getting Damage
  (`/Engine/EditorBlueprintResources/ActorMacros.Switch Has Authority`
    (:`Authority`
      (if (`self.ActorHasTag` OtherActor "Player")
        (`self.GetDamage` OtherActor)))))

(event `self.SphereOverlap`
  (bind _returnvalue (+ (`self.K2_GetActorLocation`) (* (`self.GetActorForwardVector`) 300.0)))
  (bind _returnvalue_2 (+ (`self.K2_GetActorLocation`) (* (`self.GetActorForwardVector`) 300.0)))
  (`/Engine/EditorBlueprintResources/ActorMacros.Switch Has Authority`
    (:`Authority`
      (switch `/Game/Characters/Monsters/EnemyAI/EN_AiAttacksTypes` (`self.AttackTypes`)
        (:`NewEnumerator1`
          ;[0 0 0 1 36] HeavyAttack - WithAoeColission
          (bind _outactors (`KismetSystemLibrary.SphereOverlapActors` _returnvalue_2 100.0 (`|MakeArray` "ObjectTypeQuery3" :!type "EObjectTypeQuery Enum") null (`|MakeArray` self :!type "Actor Object Reference")))
          ;;[1 0.08657 0] DebugOnly-Offline
          (`KismetSystemLibrary.DrawDebugSphere` _returnvalue_2 100.0 12 (struct :`R` 1.0 :`B` 0.155394 :`A` 1.0) 2.0 1.0)
          (for _array_element _outactors
            (if (`self.ActorHasTag` _array_element "Player")
              (`self.GetDamage` _array_element)
              (bind _ascharacter (cast `Character` _array_element :!pure true))
              ;;[1 0.9394 0.4187] KnockBack
              (`self.LaunchCharacter` _ascharacter (* (`KismetMathLibrary.MakeVector` (.x (`KismetMathLibrary.GetDirectionUnitVector` (`self.K2_GetActorLocation` _ascharacter) (`self.K2_GetActorLocation`))) (.y (`KismetMathLibrary.GetDirectionUnitVector` (`self.K2_GetActorLocation` _ascharacter) (`self.K2_GetActorLocation`))) (+ (.z (`KismetMathLibrary.GetDirectionUnitVector` (`self.K2_GetActorLocation` _ascharacter) (`self.K2_GetActorLocation`))) 1.0)) 500.0) false false))))
        (:`NewEnumerator3`
          ;[0 0 0 1 36] Charge Attack - WithAoeColission
          (bind _outactors_2 (`KismetSystemLibrary.SphereOverlapActors` _returnvalue 100.0 (`|MakeArray` "ObjectTypeQuery3" :!type "EObjectTypeQuery Enum") null (`|MakeArray` self :!type "Actor Object Reference")))
          ;;[1 0.08657 0] DebugOnly-Offline
          (`KismetSystemLibrary.DrawDebugSphere` _returnvalue 100.0 12 (struct :`R` 1.0 :`B` 0.155394 :`A` 1.0) 2.0 1.0)
          (for _array_element_2 _outactors_2
            (if (`self.ActorHasTag` _array_element_2 "Player")
              (`self.GetDamage` _array_element_2)
              (bind _ascharacter_2 (cast `Character` _array_element_2 :!pure true))
              ;;[1 0.9394 0.4187] KnockBack
              (`self.LaunchCharacter` _ascharacter_2 (* (`KismetMathLibrary.MakeVector` (.x (`KismetMathLibrary.GetDirectionUnitVector` (`self.K2_GetActorLocation` _ascharacter_2) (`self.K2_GetActorLocation`))) (.y (`KismetMathLibrary.GetDirectionUnitVector` (`self.K2_GetActorLocation` _ascharacter_2) (`self.K2_GetActorLocation`))) (+ (.z (`KismetMathLibrary.GetDirectionUnitVector` (`self.K2_GetActorLocation` _ascharacter_2) (`self.K2_GetActorLocation`))) 1.0)) 500.0) false false))))))))

(event `self.DoRangeAttack`
  ;[1 1 1] RangeAttack
  (`|SpawnActorFromClass` "/Game/Characters/Monsters/EnemyAI/BP_Projectile_Base.BP_Projectile_Base_C" (`SceneComponent.K2_GetComponentToWorld` (`self.SpawnProjectile`)) "AlwaysSpawn" "OverrideRootScale" self 0.0 null))

(fn `AttackPercent`
  (params (Percent :type "Float (double-precision)"))
  (returns (Return :type Boolean))
  (return (select `bool` (== Percent 0.0) :`false` (<= (`KismetMathLibrary.RandomFloatInRange` 0.0 100.0) Percent))))

(fn `ClearPlayerTarget`)

(fn `DistanceCheck`
  (if (> (`self.GetDistanceTo` self (`self.Target`)) 1500.0)
    (`self.ClearPlayerTarget`)
    (`KismetSystemLibrary.K2_ClearAndInvalidateTimerHandle` (`self.DistanceHandle`))))

(fn `GetAttackType`
  (returns (AttackTypes :type "/Game/Characters/Monsters/EnemyAI/EN_AiAttacksTypes Enum"))
  (return (`self.AttackTypes`)))

(fn `GetCombatState`
  (returns (InCombat :type Boolean))
  (return (`self.InCombat`)))

(fn `GetDamage`
  (params (HitPlayer :type "Actor Object Reference"))
  (switch `/Game/Characters/Monsters/EnemyAI/EN_AiAttacksTypes` (`self.AttackTypes`)
    (:`NewEnumerator0`
      (`GameplayStatics.ApplyDamage` HitPlayer (`self.LightAttack_Damage`) null self "/Script/Engine.DamageType"))
    (:`NewEnumerator1`
      (`GameplayStatics.ApplyDamage` HitPlayer (`self.HeavyAttack_Damage`) null self "/Script/Engine.DamageType"))
    (:`NewEnumerator2`
      (`GameplayStatics.ApplyDamage` HitPlayer (`self.RangeAttack_Damage`) null self "/Script/Engine.DamageType"))
    (:`NewEnumerator3`
      (`GameplayStatics.ApplyDamage` HitPlayer (`self.ChargeAttack_Damage`) null self "/Script/Engine.DamageType"))
    (:`NewEnumerator4`
      (`GameplayStatics.ApplyDamage` HitPlayer (`self.SpecialAttack_Damage`) null self "/Script/Engine.DamageType"))))

(fn `GetMontage`
  (params (Montages :type "Array of AnimMontage Object Reference"))
  (returns (Output :type "AnimMontage Object Reference"))
  (return (`|GetArrayItem` Montages (`KismetMathLibrary.RandomIntegerInRange` 0 (- (`KismetArrayLibrary.Array_Length` Montages) 1)))))

(fn `GetPlayerTarget`
  (returns (Target :type "Actor Object Reference"))
  (return (`self.Target`)))

(fn `MovmentState`
  (params (Movement :type "/Game/Characters/Monsters/EnemyAI/EN_AiState Enum" :default "NewEnumerator0"))
  (set `CharacterMovementComponent.MaxWalkSpeed` 600.0 (`self.CharacterMovement`)))

(fn `PickAttack`
  (params (PlayerDistance :type "Float (double-precision)"))
  (returns (Lenght :type "Float (double-precision)"))
  (bind _output (`self.GetMontage` (`self.ChargeAttack`)))
  (bind _output_2 (`self.GetMontage` (`self.BasicMelleAttack`)))
  (bind _output_3 (`self.GetMontage` (`self.RangeAttack`)))
  (bind _output_4 (`self.GetMontage` (`self.HeavyMelleAttack`)))
  (if (<= PlayerDistance (`self.MelleAttackDistance`))
    (if (`self.AttackPercent` 65.0)
      ;[0 0 0] LightAttack
      (set `self.AttackTypes` "NewEnumerator0")
      (`self.Multiplayer_PlayMontage` (`self.Mesh`) _output_2)
      (bind _returnvalue (`AnimSequenceBase.GetPlayLength` _output_2))
      (return _returnvalue)
      (else
        ;[0 0 0] HeavyAttack
        (set `self.AttackTypes` "NewEnumerator1")
        (`self.Multiplayer_PlayMontage` (`self.Mesh`) _output_4)
        (bind _returnvalue_2 (`AnimSequenceBase.GetPlayLength` _output_4))
        (return _returnvalue_2)))
    (elif (<= PlayerDistance (`self.RangeAttackDistance`))
      ;[1 0.09129 0] ChargedAttack
      (set `self.AttackTypes` "NewEnumerator3")
      (`self.Multiplayer_PlayMontage` (`self.Mesh`) _output)
      (bind _returnvalue_3 (`AnimSequenceBase.GetPlayLength` _output))
      (return _returnvalue_3)
      (else
        ;[1 0.09129 0] RangeAttack
        (set `self.AttackTypes` "NewEnumerator2")
        (`self.Multiplayer_PlayMontage` (`self.Mesh`) _output_3)
        (bind _returnvalue_4 (`AnimSequenceBase.GetPlayLength` _output_3))
        (return _returnvalue_4)))))

(fn `UserConstructionScript`)