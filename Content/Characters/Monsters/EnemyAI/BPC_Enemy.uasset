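; AI controller for enemies that turns sight and damage perception of BP_MinaChar into blackboard target and attack keys.
; Sight adds players to TargetsOnSight with stimulus strength as aggro, then sets Target to the highest.
; Damage adds new attackers without retargeting; its aggro increase for known ones only edits an array copy.
; Eye viewpoint comes from a mesh socket, and canAttack? starts true on BeginPlay.
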(event `self.ReceiveBeginPlay`
  (`self.UpdateCanAttackKey` true))

(event `self.AIPerception.OnTargetPerceptionUpdated`
  (params (Actor :type "Actor Object Reference") (Stimulus :type "AIStimulus Structure"))
  (bind _returnvalue (`AIPerceptionSystem.GetSenseClassForStimulus` Stimulus))
  (`KismetSystemLibrary.PrintString` (`KismetTextLibrary.Conv_TextToString` (`|FormatText` "Stimuli Class Name: {StimulusName}" (`KismetSystemLibrary.GetClassDisplayName` _returnvalue))))
  (if (== _returnvalue "/Script/AIModule.AISense_Sight")
    (`self.OnSightPerceptionUpdated` Actor Stimulus)
    (elif (== _returnvalue "/Script/AIModule.AISense_Damage")
      (`self.OnDamagePerceptionUpdated` Actor Stimulus))))

(fn `BPGetActorEyesViewPoint`
  (returns (out_Location :type "Vector Structure") (out_Rotation :type "Rotator Structure"))
  (bind _asbp_enemy (cast `/Game/Characters/Monsters/EnemyAI/BP_Enemy` (`self.K2_GetPawn`)))
  (bind (_returnvalue_location _returnvalue_rotation) (`KismetMathLibrary.BreakTransform` (`SceneComponent.GetSocketTransform` (`Character.Mesh` _asbp_enemy) (`self.Eye Socked Name`) "RTS_World")))
  (return _returnvalue_location _returnvalue_rotation))

(fn `GetHighestAggro`
  (params (Targets :type "Set of /Game/Characters/Monsters/EnemyAI/S_Target Structure"))
  (returns (Player :type "/Game/Characters/Mina/BP_MinaChar Object Reference"))
  (locals (HighestAggro :type "Float (double-precision)") (PlayerIndex :type Integer))
  (bind _result (`BlueprintSetLibrary.Set_ToArray` Targets))
  (for (_array_element _array_index) _result
    (bind (_player _aggro) (break `/Game/Characters/Monsters/EnemyAI/S_Target` _array_element))
    (if (> _aggro (`local.HighestAggro`))
      (set `local.HighestAggro` _aggro)
      (set `local.PlayerIndex` _array_index)))
  (bind _output_player (break `/Game/Characters/Monsters/EnemyAI/S_Target` (`|GetArrayItem` _result (`local.PlayerIndex`))))
  (return _output_player))

(fn `OnDamagePerceptionUpdated`
  (params (Actor :type "Actor Object Reference") (Stimuli :type "AIStimulus Structure"))
  (if (`.bSuccessfullySensed` (break `AIStimulus` Stimuli))
    (bind _asbp_mina_char (cast `/Game/Characters/Mina/BP_MinaChar` Actor))
    (bind _result (`BlueprintSetLibrary.Set_ToArray` (`self.TargetsOnSight`)))
    (for (_array_element _array_index) _
      (bind (_player _aggro) (break `/Game/Characters/Monsters/EnemyAI/S_Target` _array_element))
      (if (== _asbp_mina_char _player)
        (`KismetArrayLibrary.Array_Set` _result _array_index (make `/Game/Characters/Monsters/EnemyAI/S_Target` _player (+ _aggro 10.0)))
        (return)))
    (`BlueprintSetLibrary.Set_Add` (`self.TargetsOnSight`) (make `/Game/Characters/Monsters/EnemyAI/S_Target` _asbp_mina_char 10.0))
    (return)))

(fn `OnSightPerceptionUpdated`
  (params (Actor :type "Actor Object Reference") (Stimuli :type "AIStimulus Structure"))
  (bind (_age _expirationage _strength _stimuluslocation _receiverlocation _tag _bsuccessfullysensed) (break `AIStimulus` Stimuli))
  (bind _targetsonsight (`self.TargetsOnSight`))
  (if _bsuccessfullysensed
    (bind _asbp_mina_char (cast `/Game/Characters/Mina/BP_MinaChar` Actor))
    (`BlueprintSetLibrary.Set_Add` _targetsonsight (make `/Game/Characters/Monsters/EnemyAI/S_Target` _asbp_mina_char _strength))
    (bind _player (`self.GetHighestAggro` _targetsonsight))
    (`self.UpdateTargetKey` _player)))

(fn `UpdateCanAttackKey`
  (params (`canAttack?` :type Boolean))
  (`BlackboardComponent.SetValueAsBool` (`AIBlueprintHelperLibrary.GetBlackboard` null) "canAttack?" `canAttack?`))

(fn `UpdateHasAgroKey`
  (params (HasAgro :type Boolean))
  (`BlackboardComponent.SetValueAsBool` (`self.Blackboard`) "HasAgro" HasAgro))

(fn `UpdateTargetKey`
  (params (PlayerRef :type "/Game/Characters/Mina/BP_MinaChar Object Reference"))
  (`BlackboardComponent.SetValueAsObject` (`self.Blackboard`) "Target" PlayerRef))

(fn `UserConstructionScript`)