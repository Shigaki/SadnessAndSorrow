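; Base enemy character Blueprint that takes damage, shows floating combat text and attacks players in melee.
; AnyDamage reduces health, flagging a hit reaction while alive, otherwise disabling movement and expiring the actor shortly after.
; CheckHit damages Player-tagged pawns in a debug-drawn sphere, gating attacks through the BPC_Enemy AI controller during a timed cooldown.
; Blackboard helpers manage target and aggro; TargetLockon toggles a marker, while sphere-vision targeting is disconnected.
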(event `self.ReceiveBeginPlay`
  (set `self.CurHealth` (`self.MaxHealth`))
  ;[1 0 0.006678] Load_Combat_Text
  (set `self.CombatText` (cast `/Game/UI/CombatInfo/W_CombatText` (`WidgetComponent.GetUserWidgetObject` (`self.FloatingCombatText`)) :!pure true)))

(event `self.ReceiveAnyDamage`
  (params (Damage :type "Float (single-precision)") (DamageType :type "DamageType Object Reference") (InstigatedBy :type "Controller Object Reference") (DamageCauser :type "Actor Object Reference"))
  ;[1 0.01872 0] On Damage
  (`self.Multi_CombatText` Damage)
  (bind _isalive_ (`self.TakeDamage` Damage))
  (if _isalive_
    (`self.SetReactToHit` true)
    (else
      (`CharacterMovementComponent.DisableMovement` (`self.CharacterMovement`))
      (set `self.isAlive` false)
      (`/Engine/EditorBlueprintResources/StandardMacros.DoOnce` false
        (:`Completed`
          (`self.SetLifeSpan` 2.0))))))

(event `Multi_CombatText`
  (params (DamageAmount :type "Float (double-precision)") (DamageType :type "/Game/GlobalSettings/Enums/E_DamageType Enum" :default "NewEnumerator0"))
  ;[0.3281 0.002984 0] Play CombatText
  (`/Game/UI/CombatInfo/W_CombatText.Play_CombatText` (`self.CombatText`) DamageAmount DamageType))

(event `self.SphereVision.OnComponentBeginOverlap`
  (params (OverlappedComponent :type "PrimitiveComponent Object Reference") (OtherActor :type "Actor Object Reference") (OtherComp :type "PrimitiveComponent Object Reference") (OtherBodyIndex :type Integer) (bFromSweep :type Boolean) (SweepResult :type "HitResult Structure (by ref)")))

(event `self.SphereVision.OnComponentEndOverlap`
  (params (OverlappedComponent :type "PrimitiveComponent Object Reference") (OtherActor :type "Actor Object Reference") (OtherComp :type "PrimitiveComponent Object Reference") (OtherBodyIndex :type Integer)))

(event `CheckHit`
  (bind _returnvalue (`SceneComponent.K2_GetComponentLocation` (`self.DamageArrow`)))
  (bind _asbpc_enemy (cast `/Game/Characters/Monsters/EnemyAI/BPC_Enemy` (`AIBlueprintHelperLibrary.GetAIController` self)))
  (`/Game/Characters/Monsters/EnemyAI/BPC_Enemy.UpdateCanAttackKey` _asbpc_enemy false)
  (bind (_outactors _returnvalue_2) (`KismetSystemLibrary.SphereOverlapActors` _returnvalue (`self.damageRadius`) (`|MakeArray` "ObjectTypeQuery3" :!type "EObjectTypeQuery Enum") null (`|MakeArray` self :!type "Actor Object Reference")))
  (`KismetSystemLibrary.DrawDebugSphere` _returnvalue 100.0 12 (struct :`R` 0.600554 :`B` 1.0 :`A` 1.0) 2.0)
  (if _returnvalue_2
    (for _array_element _outactors
      (if (`self.ActorHasTag` _array_element "Player")
        (`GameplayStatics.ApplyDamage` _array_element 299.0 (`self.GetController`) self "/Script/Engine.DamageType"))))
  (set `CharacterMovementComponent.MaxWalkSpeed` 300.0 (`self.CharacterMovement`))
  (`KismetSystemLibrary.Delay` 4.0)
  (bind _asbpc_enemy_2 (cast `/Game/Characters/Monsters/EnemyAI/BPC_Enemy` (`AIBlueprintHelperLibrary.GetAIController` self)))
  (`/Game/Characters/Monsters/EnemyAI/BPC_Enemy.UpdateCanAttackKey` _asbpc_enemy_2 true)
  (set `CharacterMovementComponent.MaxWalkSpeed` 150.0 (`self.CharacterMovement`)))

(event `/Game/GlobalSettings/Interfaces/BPI_TargetLock.TargetLockOn`
  (bind _targetvisual (`self.TargetVisual`))
  (`/Engine/EditorBlueprintResources/StandardMacros.FlipFlop`
    (:`A`
      (`SceneComponent.SetHiddenInGame` _targetvisual false false))
    (:`B`
      (`SceneComponent.SetHiddenInGame` _targetvisual true false))))

(fn `ClearAgro`
  (`BlackboardComponent.ClearValue` (`AIBlueprintHelperLibrary.GetBlackboard` (`AIBlueprintHelperLibrary.GetAIController` self)) "HasAgro"))

(fn `ClearTarget`
  (`BlackboardComponent.ClearValue` (`AIBlueprintHelperLibrary.GetBlackboard` (`AIBlueprintHelperLibrary.GetAIController` self)) "Target"))

(fn `GetDistanceFromTarget`
  (returns (distance :type "Float (double-precision)"))
  (return (`self.GetDistanceTo` (`self.GetTarget`))))

(fn `GetTarget`
  (returns (Target :type "Actor Object Reference"))
  (bind _asactor (cast `Actor` (`BlackboardComponent.GetValueAsObject` (`AIBlueprintHelperLibrary.GetBlackboard` (`AIBlueprintHelperLibrary.GetAIController` self)) "Target"))
    (:`then`
      (return _asactor))
    (:`CastFailed`
      (return null))))

(fn `SetCanAttack`
  (params (newTarget :type Boolean)))

(fn `SetReactToHit`
  (params (react :type Boolean))
  (set `self.reactToHit` react)
  (`self.SetCanAttack` (not react)))

(fn `SetTarget`
  (params (newTarget :type "Object Object Reference"))
  (`BlackboardComponent.SetValueAsObject` (`AIBlueprintHelperLibrary.GetBlackboard` (`AIBlueprintHelperLibrary.GetAIController` self)) "Target" newTarget))

(fn `SpawnDamageTooltip`
  (params (Amount :type "Float (double-precision)") (Color :type "Color Structure"))
  (returns (Success :type Boolean))
  (locals (NewLocalVar_0 :type "Object Object Reference"))
  (bind _returnvalue (`|SpawnActorFromClass` "/Game/UI/CombatInfo/BP_CombText.BP_CombText_C" (`KismetMathLibrary.MakeTransform` (`SceneComponent.K2_GetComponentLocation` (`self.Mesh`)) (`self.K2_GetActorRotation` (`GameplayStatics.GetPlayerPawn` 0))) "Undefined" "OverrideRootScale" null null))
  (bind _textrender (`/Game/UI/CombatInfo/BP_CombText.TextRender` _returnvalue))
  (`TextRenderComponent.K2_SetText` _textrender (`KismetTextLibrary.Conv_DoubleToText` Amount "HalfToEven"))
  (`TextRenderComponent.SetTextRenderColor` _textrender Color)
  (return true))

(fn `TakeDamage`
  (params (Amount :type "Float (double-precision)"))
  (returns (`isAlive?` :type Boolean))
  (bind _output_get (set `self.CurHealth` (- (`self.CurHealth`) Amount)))
  (return (> _output_get 0.0)))

(fn `UserConstructionScript`)