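; BP_Projectile_Base is a base enemy projectile that damages actors tagged Player on contact.
; On the authority only, the sphere's overlap sets GetHit, applies damage with the projectile's owner as causer, then destroys the projectile.
; On destruction, a set GetHit flag triggers MultiSpawn, an event left empty in this Blueprint.
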(event `self.Sphere.OnComponentBeginOverlap`
  (params (OverlappedComponent :type "PrimitiveComponent Object Reference") (OtherActor :type "Actor Object Reference") (OtherComp :type "PrimitiveComponent Object Reference") (OtherBodyIndex :type Integer) (bFromSweep :type Boolean) (SweepResult :type "HitResult Structure (by ref)"))
  (`/Engine/EditorBlueprintResources/ActorMacros.Switch Has Authority`
    (:`Authority`
      (if (`self.ActorHasTag` OtherActor "Player")
        (set `self.GetHit` true)
        (`GameplayStatics.ApplyDamage` null (`self.Base Damage`) null (`self.GetOwner`))
        (`self.K2_DestroyActor`)))))

(event `self.ReceiveDestroyed`
  (if (`self.GetHit`)
    (`self.MultiSpawn`)))

(event `MultiSpawn`)

(fn `UserConstructionScript`)