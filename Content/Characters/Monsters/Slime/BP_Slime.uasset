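; BP_Slime is the slime monster character, which feeds AI perception results to its BPC_Slime controller.
; Sensing an actor cancels any pending lost-target timer and sets the controller's target and line-of-sight keys.
; Losing sight clears line of sight at once, then a three-second timer clears the target, giving a grace period before the slime forgets it.
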(event `self.AIPerception.OnTargetPerceptionUpdated`
  (params (Actor :type "Actor Object Reference") (Stimulus :type "AIStimulus Structure"))
  (set `self.PerceivedActor` Actor)
  (if (`.bSuccessfullySensed` (break `AIStimulus` Stimulus))
    (`KismetSystemLibrary.K2_ClearAndInvalidateTimerHandle` (`self.TargetLostTimer`))
    (bind _asbpc_slime (cast `/Game/Characters/Monsters/Slime/BPC_Slime` (`self.GetController`)))
    (`/Game/Characters/Monsters/Slime/BPC_Slime.UpdateTargetActorKey` _asbpc_slime (`self.PerceivedActor`))
    (`/Game/Characters/Monsters/Slime/BPC_Slime.UpdateHasLineOfSightKey` _asbpc_slime true)
    (else
      (bind _returnvalue (`KismetSystemLibrary.K2_SetTimerDelegate` (delegate `TargetLost`) 3.0))
      (set `self.TargetLostTimer` _returnvalue)
      (bind _asbpc_slime_2 (cast `/Game/Characters/Monsters/Slime/BPC_Slime` (`self.GetController`)))
      (`/Game/Characters/Monsters/Slime/BPC_Slime.UpdateHasLineOfSightKey` _asbpc_slime_2 false))))

(event `TargetLost`
  (set `self.PerceivedActor` null)
  (bind _asbpc_slime (cast `/Game/Characters/Monsters/Slime/BPC_Slime` (`self.GetController`)))
  (`/Game/Characters/Monsters/Slime/BPC_Slime.UpdateTargetActorKey` _asbpc_slime null))

(fn `UserConstructionScript`)