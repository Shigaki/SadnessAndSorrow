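; BP_Boar is a boar monster character that extends a parent class with its own melee and special attacks.
; On BeginPlay it runs the parent logic, sets its close and long attack ranges and damage radius, and disables capsule physics simulation.
; BasicAttack and SpecialAttack each snap the boar's yaw toward a valid target, then play the matching montage, even without a target.
; A leftover move-to-target node is never executed.
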(event `self.ReceiveBeginPlay`
  (`parent.ReceiveBeginPlay`)
  (set `self.CloseRangeAttackDistance` 100.0)
  (set `self.LongRangeAttackDistance` 600.0)
  (set `self.damageRadius` 25.0)
  (`PrimitiveComponent.SetSimulatePhysics` (`self.CapsuleComponent`) false))

(event `BasicAttack`
  (params (Target :type "Actor Object Reference"))
  (bind (_returnvalue_roll _returnvalue_pitch _returnvalue_yaw) (`KismetMathLibrary.BreakRotator` (`KismetMathLibrary.FindLookAtRotation` (`self.K2_GetActorLocation`) (`self.K2_GetActorLocation` Target))))
  (`|ExecutionSequence`
    (:`then_0`
      (`/Engine/EditorBlueprintResources/StandardMacros.IsValid` Target
        (:`Is Valid`
          (`self.K2_SetActorRotation` (`KismetMathLibrary.MakeRotator` 0.0 0.0 _returnvalue_yaw)))))
    (:`then_1`
      (`self.PlayAnimMontage` "/Game/Characters/Monsters/Boar/Boar_BasicAttack.Boar_BasicAttack"))))

(event `SpecialAttack`
  (params (Target :type "Actor Object Reference"))
  (bind (_returnvalue_roll _returnvalue_pitch _returnvalue_yaw) (`KismetMathLibrary.BreakRotator` (`KismetMathLibrary.FindLookAtRotation` (`self.K2_GetActorLocation`) (`self.K2_GetActorLocation` Target))))
  (`|ExecutionSequence`
    (:`then_0`
      (`/Engine/EditorBlueprintResources/StandardMacros.IsValid` Target
        (:`Is Valid`
          (`self.K2_SetActorRotation` (`KismetMathLibrary.MakeRotator` 0.0 0.0 _returnvalue_yaw)))))
    (:`then_1`
      (`self.PlayAnimMontage` "/Game/Characters/Monsters/Boar/Boar_SpecialAttack.Boar_SpecialAttack"))))

(fn `UserConstructionScript`
  (`parent.UserConstructionScript`))