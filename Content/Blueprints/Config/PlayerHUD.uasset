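; PlayerHUD shows the player character's health, mana and stamina through a StatsBar widget.
; On BeginPlay it adds the widget to the viewport, casts the player character to BP_MinaChar and caches its three maximum values once.
; Tick polls the current values while the character is valid, and per-stat functions normalize them against the cached maximums before passing them to the widget.
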(event `self.ReceiveBeginPlay`
  (bind _returnvalue (`|CreateWidget` "/Game/UI/PlayerInfo/StatsBar.StatsBar_C" (`GameplayStatics.GetPlayerController` 0)))
  (bind _output_get (set `self.StatsBarRef` _returnvalue))
  (`UserWidget.AddToViewport` _output_get 0)
  (bind _asbp_mina_char (cast `/Game/Characters/Mina/BP_MinaChar` (`GameplayStatics.GetPlayerCharacter` 0)))
  (set `self.CharacterRef` _asbp_mina_char)
  (`self.Init`))

(event `Init`
  (bind _characterref (`self.CharacterRef`))
  (set `self.MaxHealth` (`/Game/Characters/Mina/BP_MinaChar.MaxHealth` _characterref))
  (set `self.MaxMana` (`/Game/Characters/Mina/BP_MinaChar.MaxMana` _characterref))
  (set `self.MaxStamina` (`/Game/Characters/Mina/BP_MinaChar.MaxStamina` _characterref)))

(event `self.ReceiveTick`
  (params (DeltaSeconds :type "Float (single-precision)"))
  (bind _characterref (`self.CharacterRef`))
  (`/Engine/EditorBlueprintResources/StandardMacros.IsValid` (`self.CharacterRef`)
    (:`Is Valid`
      (`self.UpdateHealth` (`/Game/Characters/Mina/BP_MinaChar.CurHealth` _characterref))
      (`self.UpdateStamina` (`/Game/Characters/Mina/BP_MinaChar.CurStamina` _characterref))
      (`self.UpdateMana` (`/Game/Characters/Mina/BP_MinaChar.CurMana` _characterref)))))

(fn `UpdateHealth`
  (params (InPercent :type "Float (double-precision)"))
  (`/Game/UI/PlayerInfo/StatsBar.UpdateHealth` (`self.StatsBarRef`) (`KismetMathLibrary.NormalizeToRange` InPercent 0.0 (`self.MaxHealth`))))

(fn `UpdateMana`
  (params (InPercent :type "Float (double-precision)"))
  (`/Game/UI/PlayerInfo/StatsBar.UpdateMana` (`self.StatsBarRef`) (`KismetMathLibrary.NormalizeToRange` InPercent 0.0 (`self.MaxMana`))))

(fn `UpdateStamina`
  (params (InPercent :type "Float (double-precision)"))
  (`/Game/UI/PlayerInfo/StatsBar.UpdateStamina` (`self.StatsBarRef`) (`KismetMathLibrary.NormalizeToRange` InPercent 0.0 (`self.MaxStamina`))))

(fn `UserConstructionScript`)