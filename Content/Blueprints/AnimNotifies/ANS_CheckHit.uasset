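; ANS_CheckHit is an anim notify state that performs weapon hit detection during its animation window.
; Each tick, it sphere-traces on the Camera channel from the owning Character's main-hand weapon socket a short distance along the actor's forward vector, drawing debug for one frame.
; It applies fixed damage to the hit actor every tick, with no tracking of actors already hit.
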(fn `Received_NotifyTick`
  (params (MeshComp :type "SkeletalMeshComponent Object Reference") (Animation :type "AnimSequenceBase Object Reference") (FrameDeltaTime :type "Float (double-precision)"))
  (returns (ReturnValue :type Boolean))
  (bind _ascharacter (cast `Character` (`ActorComponent.GetOwner` MeshComp)))
  (bind _returnvalue (`SceneComponent.GetSocketLocation` (`Character.Mesh` _ascharacter) "main_hand_weapon_socket"))
  (bind _outhit (`KismetSystemLibrary.SphereTraceSingle` :`WorldContextObject` MeshComp :`Start` _returnvalue :`End` (+ _returnvalue (* (`KismetMathLibrary.GetForwardVector` (`Actor.K2_GetActorRotation` _ascharacter)) 100.0)) :`Radius` 40.0 :`TraceChannel` "TraceTypeQuery2" :`DrawDebugType` "ForOneFrame"))
  (`GameplayStatics.ApplyDamage` (`.HitActor` (`GameplayStatics.BreakHitResult` _outhit)) 10.0 null _ascharacter "/Script/Engine.DamageType")
  (return false))