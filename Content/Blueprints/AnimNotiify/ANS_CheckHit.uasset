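; Anim notify state that performs melee hit detection for MinaCharBP during the active window of an animation.
; Each notify tick sphere-traces on the Camera channel from the mesh's MainWeaponSocket along the character's forward vector, with debug drawing.
; The hit actor receives fixed damage with the character as causer.
; It keeps no record of previous hits, so one target can take damage on successive ticks.
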(fn `Received_NotifyTick`
  (params (MeshComp :type "SkeletalMeshComponent Object Reference") (Animation :type "AnimSequenceBase Object Reference") (FrameDeltaTime :type "Float (double-precision)"))
  (returns (ReturnValue :type Boolean))
  (bind _asmina_char_bp (cast `/Game/Characters/Mina/MinaCharBP` (`ActorComponent.GetOwner` MeshComp)))
  (bind _returnvalue (`SceneComponent.GetSocketLocation` (`Character.Mesh` _asmina_char_bp) "MainWeaponSocket"))
  (bind _outhit (`KismetSystemLibrary.SphereTraceSingle` :`WorldContextObject` MeshComp :`Start` _returnvalue :`End` (+ _returnvalue (* (`KismetMathLibrary.GetForwardVector` (`Actor.K2_GetActorRotation` _asmina_char_bp)) 100.0)) :`Radius` 40.0 :`TraceChannel` "TraceTypeQuery2" :`DrawDebugType` "ForOneFrame"))
  (`GameplayStatics.ApplyDamage` (`.HitActor` (`GameplayStatics.BreakHitResult` _outhit)) 10.0 null _asmina_char_bp "/Script/Engine.DamageType")
  (return false))