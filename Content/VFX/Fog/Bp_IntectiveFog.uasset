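; Volumetric fog volume actor that renders shaped, height-aware fog through a Niagara system and a dynamic M_FogParticle material, set up entirely in the construction script.
; It sizes the box, hands material and size to Niagara, then pushes shape, fog type, color and noise settings to the material.
; A downward orthographic scene capture renders selected actors into HeightRT, which feeds the material.
; The render target created as FogHeight is unused.
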(fn `Call`
  (`SceneCaptureComponent2D.CaptureScene` (`self.HeighCapture`))
  (return))

(fn `HeightSet`
  (bind (_returnvalue_x _returnvalue_y _returnvalue_z) (`KismetMathLibrary.BreakVector` (`self.K2_GetActorLocation`)))
  (bind (_volumesize_x _volumesize_y _volumesize_z) (`KismetMathLibrary.BreakVector` (`self.VolumeSize`)))
  (bind _heighcapture (`self.HeighCapture`))
  (bind (_volumesize_x_2 _volumesize_y_2 _volumesize_z_2) (`KismetMathLibrary.BreakVector` (`self.VolumeSize`)))
  (`SceneComponent.K2_SetWorldLocationAndRotation` _heighcapture (`KismetMathLibrary.MakeVector` _returnvalue_x _returnvalue_y (+ _returnvalue_z (/ _volumesize_z_2 2.0))) (struct :`Pitch` -90.0 :`Roll` -90.0) false false)
  (set `SceneCaptureComponent2D.OrthoWidth` (`KismetMathLibrary.FMax` (`KismetMathLibrary.FMax` _volumesize_x _volumesize_y) _volumesize_z) _heighcapture)
  (set `SceneCaptureComponent2D.TextureTarget` (`self.HeightRT`) _heighcapture)
  (set `SceneCaptureComponent.ShowOnlyActors` (`self.HeightActors`) _heighcapture)
  (`self.Call`))

(fn `Niagara Variables`
  (bind _ns_fog (`self.NS_Fog`))
  (bind (_volumesize_x _volumesize_y _volumesize_z) (`KismetMathLibrary.BreakVector` (`self.VolumeSize`)))
  (`NiagaraComponent.SetVariableMaterial` _ns_fog "FogMid" (`self.FogMid`))
  (`NiagaraComponent.SetVariableFloat` _ns_fog "VolumeSizeMax" (* (`KismetMathLibrary.FMax` (`KismetMathLibrary.FMax` _volumesize_x _volumesize_y) _volumesize_z) 2.0))
  (return))

(fn `UserConstructionScript`
  (bind _returnvalue (`KismetMaterialLibrary.CreateDynamicMaterialInstance` "/Game/VFX/Fog/M_FogParticle.M_FogParticle"))
  (set `self.FogMid` _returnvalue)
  (bind _returnvalue_2 (`KismetRenderingLibrary.CreateRenderTarget2D` 256 256 "RTF_R32f"))
  (set `self.FogHeight` _returnvalue_2)
  (`BoxComponent.SetBoxExtent` (`self.Box`) (/ (`self.VolumeSize`) 2.0) true)
  (`self.Niagara Variables`)
  (`self.VolumeControl`)
  (`self.HeightSet`))

(fn `VolumeControl`
  (bind _fogmid (`self.FogMid`))
  ;[1 1 1] Size Variables
  (`MaterialInstanceDynamic.SetVectorParameterValue` _fogmid "ShapeType" (select `/Game/VFX/Fog/E_Fog_ShapeType` (`self.ShapeType`) :`NewEnumerator0` (struct :`R` 1.0) :`NewEnumerator1` (struct :`G` 1.0) :`NewEnumerator2` (struct :`B` 1.0) :`NewEnumerator3` (struct :`A` 1.0) :!type "LinearColor Structure"))
  (`MaterialInstanceDynamic.SetVectorParameterValue` _fogmid "VolumeSize" (`KismetMathLibrary.Conv_VectorToLinearColor` (`self.VolumeSize`)))
  (`MaterialInstanceDynamic.SetScalarParameterValue` _fogmid "Falloff" (`self.FallOff`))
  (`MaterialInstanceDynamic.SetTextureParameterValue` _fogmid "Texture2D" (`self.Texture2D`))
  (`MaterialInstanceDynamic.SetTextureParameterValue` _fogmid "VolumetricTexture" (`self.VolumetricTexture`))
  ;[1 1 1] HeighField
  (`MaterialInstanceDynamic.SetScalarParameterValue` _fogmid "GlobalFalloff" (`self.GlobalFallOff`))
  (`MaterialInstanceDynamic.SetTextureParameterValue` _fogmid "HeightRT" (`self.HeightRT`))
  (`MaterialInstanceDynamic.SetVectorParameterValue` _fogmid "FogType" (select `/Game/VFX/Fog/E_Fog_Heigh` (`self.HeighType`) :`NewEnumerator0` (struct :`R` 1.0) :`NewEnumerator1` (struct :`G` 1.0) :`NewEnumerator2` (struct :`B` 1.0) :`NewEnumerator3` (struct :`A` 1.0) :!type "LinearColor Structure"))
  (`MaterialInstanceDynamic.SetScalarParameterValue` _fogmid "HeightSTR" (`self.HeighSTR`))
  ;[1 1 1] Fog Settings
  (`MaterialInstanceDynamic.SetScalarParameterValue` _fogmid "GlobalExtinction" (`self.GlobalExtinction`))
  (`MaterialInstanceDynamic.SetVectorParameterValue` _fogmid "Fog_BaseColor" (`self.Fog_BaseColor`))
  (`MaterialInstanceDynamic.SetVectorParameterValue` _fogmid "Extinction_BaseColor" (`self.Extinction_BaseColor`))
  (`MaterialInstanceDynamic.SetVectorParameterValue` _fogmid "Shadow_BaseColor" (`self.Shadow_BaseColor`))
  (`MaterialInstanceDynamic.SetScalarParameterValue` _fogmid "ShadowDensity" (`self.ShadowDensity`))
  (`MaterialInstanceDynamic.SetScalarParameterValue` _fogmid "NoiseScale" (`self.NoiseScale`))
  (`MaterialInstanceDynamic.SetScalarParameterValue` _fogmid "NoisePower" (`self.NoisePower`))
  (return))